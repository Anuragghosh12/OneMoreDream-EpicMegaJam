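; Battle game mode that sets up the top-down battle camera, gathers party and enemy units, and runs the turn queue.
; After a short delay on BeginPlay, it adds each party unit to the player controller's battle HUD.
; TurnRequest queues units uniquely, and a DoOnce gate in StartTurn starts one combat component's turn at a time, binding to its turn-ended event.
; ReadyNextTurn reopens the gate and starts the next queued turn.
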(event `self.ReceiveBeginPlay`
  (bind _returnvalue (`GameplayStatics.GetActorOfClass` "/Game/Project/Blueprints/Camera/Camera_TopDown.Camera_TopDown_C"))
  (bind _output_get (set `self.MainBattleCamera` _returnvalue))
  (`PlayerController.SetViewTargetWithBlend` (`GameplayStatics.GetPlayerController` 0) _output_get 0.0 "VTBlend_Linear" 0.0 false)
  (bind _outactors (`GameplayStatics.GetAllActorsOfClass` "/Game/Project/Blueprints/SpriteUnits/Sprite_PartyUnitBase.Sprite_PartyUnitBase_C"))
  (set `self.PartyUnits` _outactors)
  (bind _outactors_2 (`GameplayStatics.GetAllActorsOfClass` "/Game/Project/Blueprints/SpriteUnits/Sprite_EnemyUnitBase.Sprite_EnemyUnitBase_C"))
  (set `self.Enemy Units` _outactors_2)
  (`KismetSystemLibrary.Delay` 0.2)
  (bind _asbp_battle_player_controller (cast `/Game/Project/Blueprints/GameMode/BP_BattlePlayerController` (`GameplayStatics.GetPlayerController` 0)))
  (set `self.Battle HUD` (`/Game/Project/Blueprints/GameMode/BP_BattlePlayerController.Battle HUD` _asbp_battle_player_controller))
  (for _array_element (`self.PartyUnits`)
    (`/Game/Project/UI/Widget/BattleHUD.AddPartyUnitToHUD` (`self.Battle HUD`) _array_element)))

(event `TurnRequest`
  (params (NewParam :type "/Game/Project/Blueprints/Units/UnitBase Object Reference"))
  (`KismetArrayLibrary.Array_AddUnique` (`self.TurnOrder`) NewParam)
  (`self.StartTurn`))

(event `StartTurn`
  (bind _bp_combatcomponent (`/Game/Project/Blueprints/Units/UnitBase.BP_CombatComponent` (`|GetArrayItem` (`self.TurnOrder`))))
  (`/Engine/EditorBlueprintResources/StandardMacros.DoOnce` false :!label _label
    (:`Completed`
      (if (`KismetArrayLibrary.Array_IsValidIndex` (`self.TurnOrder`))
        (`/Game/Project/Blueprints/GameMode/BP_CombatComponent.StartUnitTurn` _bp_combatcomponent)
        (add `/Game/Project/Blueprints/GameMode/BP_CombatComponent.TurnEnded` _bp_combatcomponent (`|CreateDelegate` :!event `ReadyNextTurn`))
        (`KismetArrayLibrary.Array_Remove` (`self.TurnOrder`))
        (else
          (`self.ReadyNextTurn`))))))

(event `ReadyNextTurn`
  (`|ExecutionSequence`
    (:`then_0`
      (goto _label :!via `Reset`))
    (:`then_1`
      (if (`KismetArrayLibrary.Array_IsValidIndex` (`self.TurnOrder`))
        (`self.StartTurn`)))))

(fn `UserConstructionScript`)