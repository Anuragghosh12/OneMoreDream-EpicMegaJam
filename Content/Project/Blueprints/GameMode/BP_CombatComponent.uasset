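; Combat component for sprite units in an active-time battle, running turn timing, actions and damage math.
; A SPD-scaled timer requests turns from BP_BattleGameMode; turns open a command HUD for party units or make others attack random party members.
; Commands run melee walk-and-return, ranged damage or black/white magic spawned at the target, then restart the timer.
; Stats come from a level-keyed data table, scaled by unit modifiers.
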(event `self.ReceiveBeginPlay`
  (bind _assprite_unit_base_m (cast `/Game/Project/Blueprints/SpriteUnit/SpriteUnitBaseM` (`self.GetOwner`)))
  (bind _output_get (set `self.UnitCharacter` _assprite_unit_base_m))
  (set `self.BattlePosition` (`Actor.GetTransform` _output_get))
  (`self.BeginBattle`)
  (bind _returnvalue (`|GetDataTableRow` "/Game/Project/Blueprints/SpriteUnits/Data/BaseStatTable.BaseStatTable" (`KismetStringLibrary.Conv_StringToName` (`KismetStringLibrary.Conv_IntToString` (`self.UnitLevel`))))
    (:`then`
      (set `self.BaseUnitStats` _returnvalue))))

(event `AttackCommand`
  (if (`self.IsRangedCharacter`)
    (`self.RangedAttack`)
    (else
      (`self.MeleeAttack`))))

(event `MeleeAttack`
  (bind _battleposition_location (`KismetMathLibrary.BreakTransform` (`self.BattlePosition`)))
  ;[1 1 1] Melee
  (`|AIMoveTo` (`self.UnitCharacter`) (0.0 0.0 0.0) (`self.UnitTarget`) 100.0
    (:`then`
      (bind _actioncommandswindow (`self.ActionCommandsWindow`)
        (:`then`
          (`Widget.RemoveFromParent` _actioncommandswindow))
        (:`else`)))
    (:`OnSuccess`
      (`PaperFlipbookComponent.SetFlipbook` (`PaperCharacter.Sprite` (`self.UnitCharacter`)) (`self.AttackAnimation`))
      (`KismetSystemLibrary.Delay` 0.5)
      (`|AIMoveTo` (`self.UnitCharacter`) _battleposition_location null
        (:`OnSuccess`
          (`PaperFlipbookComponent.SetFlipbook` (`PaperCharacter.Sprite` (`self.UnitCharacter`)) (`self.IdleLeft`))
          (`KismetSystemLibrary.Delay` 0.2)
          (`self.EndUnitTurn`))))))

(event `MagicCommand`
  (params (MagicClass :type "/Game/Project/Blueprints/Abilities/MagicBase Class Reference"))
  (if (`KismetMathLibrary.ClassIsChildOf` MagicClass "/Game/Project/Blueprints/Abilities/BlackMagic/BlackMagicBase.BlackMagicBase_C")
    (`self.CastBlackMagic` MagicClass)
    (else
      (`self.CastWhiteMagic` MagicClass))))

(event `RangedAttack`
  ;[1 1 1] Ranged
  (`PaperFlipbookComponent.SetFlipbook` (`PaperCharacter.Sprite` (`self.UnitCharacter`)) (`self.AttackAnimation`))
  (bind _actioncommandswindow (`self.ActionCommandsWindow`)
    (:`then`
      (`Widget.RemoveFromParent` _actioncommandswindow))
    (:`else`
      _))
  (`self.DealDamage`)
  (`KismetSystemLibrary.Delay` 1.0)
  (`PaperFlipbookComponent.SetFlipbook` (`PaperCharacter.Sprite` (`self.UnitCharacter`)) (`self.IdleLeft`))
  (`KismetSystemLibrary.Delay` 1.0)
  (`self.EndUnitTurn`))

(event `CastBlackMagic`
  (params (BlackMagicSpell :type "/Game/Project/Blueprints/Abilities/MagicBase Class Reference"))
  (bind _unittarget (`self.UnitTarget`))
  ;[1 1 1] MagicAttack
  (`PaperFlipbookComponent.SetFlipbook` (`PaperCharacter.Sprite` (`self.UnitCharacter`)) (`self.Black Magic`))
  (bind _actioncommandswindow (`self.ActionCommandsWindow`)
    (:`then`
      (`Widget.RemoveFromParent` _actioncommandswindow))
    (:`else`
      _))
  (`|SpawnActorFromClass` BlackMagicSpell (`Actor.GetTransform` _unittarget) "Undefined" "MultiplyWithRoot" null _unittarget (`self.UnitCharacter`))
  (`KismetSystemLibrary.Delay` 0.5)
  (`PaperFlipbookComponent.SetFlipbook` (`PaperCharacter.Sprite` (`self.UnitCharacter`)) (`self.IdleLeft`))
  (`KismetSystemLibrary.Delay` 1.0)
  (`self.EndUnitTurn`))

(event `DealDamage`
  ;[1 1 1] Deal Damage
  (bind _basedamage (`self.CalculateDamage`))
  (`GameplayStatics.ApplyDamage` (`self.UnitTarget`) _basedamage null (`self.UnitCharacter`) (`self.Damage Type Class`)))

(event `CastWhiteMagic`
  (params (Ability :type "/Game/Project/Blueprints/Abilities/MagicBase Class Reference"))
  (bind _unittarget (`self.UnitTarget`))
  ;[1 1 1] White Magic
  (`PaperFlipbookComponent.SetFlipbook` (`PaperCharacter.Sprite` (`self.UnitCharacter`)) (`self.WhiteMagic`))
  (bind _actioncommandswindow (`self.ActionCommandsWindow`)
    (:`then`
      (`Widget.RemoveFromParent` _actioncommandswindow))
    (:`else`
      _))
  (`|SpawnActorFromClass` Ability (`Actor.GetTransform` _unittarget) "Undefined" "MultiplyWithRoot" null _unittarget (`self.UnitCharacter`))
  (`KismetSystemLibrary.Delay` 0.5)
  (`PaperFlipbookComponent.SetFlipbook` (`PaperCharacter.Sprite` (`self.UnitCharacter`)) (`self.IdleLeft`))
  (`KismetSystemLibrary.Delay` 1.0)
  (`self.EndUnitTurn`))

(fn `BeginBattle`
  (bind _returnvalue (`KismetSystemLibrary.K2_SetTimer` self "RequestTurn" (+ (* (- 1.0 (`KismetMathLibrary.NormalizeToRange` (`KismetMathLibrary.Conv_IntToDouble` (`.SPD_14_10281A1049C1A82E629BD8A6E5504231` (break `/Game/Project/Blueprints/SpriteUnits/Data/StatTableStruct` (`self.BaseUnitStats`)))) 0.0 255.0)) (- (`self.MaxActionTime`) (`self.MinActionTime`))) (`self.MinActionTime`))))
  (set `self.ActionTimer` _returnvalue))

(fn `CalculateBaseDamage`
  (returns (ReturnValue :type "Float (double-precision)"))
  (return (* (* (* (`.STR_19_C4EE187241AC87A86291EF8E72D0067F` (break `/Game/Project/Blueprints/SpriteUnits/Data/StatModifier` (`self.UnitStatModifier`))) (`.STR_10_C4EE187241AC87A86291EF8E72D0067F` (break `/Game/Project/Blueprints/SpriteUnits/Data/StatTableStruct` (`self.BaseUnitStats`)))) 5.0) (`KismetMathLibrary.RandomFloatInRange` 0.8 1.2))))

(fn `CalculateDamage`
  (returns (BaseDamage :type "Float (double-precision)"))
  (bind _returnvalue (`self.CalculateBaseDamage`))
  (return _returnvalue))

(fn `CalculateDamageResistance`
  (params (BaseDamage :type "Float (double-precision)"))
  (returns (NewDamage :type "Float (double-precision)"))
  (return (/ (`KismetMathLibrary.MultiplyMultiply_FloatFloat` BaseDamage 2.0) (+ BaseDamage (* (`.STA_20_2F00606542C61A77A0FC39B9887E0699` (break `/Game/Project/Blueprints/SpriteUnits/Data/StatModifier` (`self.UnitStatModifier`))) (`.STA_12_2F00606542C61A77A0FC39B9887E0699` (break `/Game/Project/Blueprints/SpriteUnits/Data/StatTableStruct` (`self.BaseUnitStats`))))))))

(fn `CalculateMagicBaseDamage`
  (params (SpellClass :type "/Game/Project/Blueprints/Abilities/MagicBase Class Reference"))
  (returns (ReturnValue :type "Float (double-precision)"))
  (bind (_abilityname _rank _spellpowertable) (defaults `Object` (`local.SpellClass`)))
  (return (* (* (`.WIS_15_DF142CDA4177344EDC574ABC8F7249F1` (break `/Game/Project/Blueprints/SpriteUnits/Data/StatTableStruct` (`self.BaseUnitStats`))) (`.WIS_23_DF142CDA4177344EDC574ABC8F7249F1` (break `/Game/Project/Blueprints/SpriteUnits/Data/StatModifier` (`self.UnitStatModifier`)))) (* (`KismetMathLibrary.Sqrt` (`BlueprintMapLibrary.Map_Find` _spellpowertable _rank)) 2.0))))

(fn `EndUnitTurn`
  (`self.TurnEnded`)
  (`self.BeginBattle`))

(fn `GetRangePosition`
  (returns (ReturnValue :type "Vector Structure"))
  (bind _returnvalue (`Actor.K2_GetActorLocation` (`self.UnitCharacter`)))
  (return (+ _returnvalue (* (`KismetMathLibrary.GetDirectionUnitVector` _returnvalue (`Actor.K2_GetActorLocation` (`self.UnitTarget`))) 500.0))))

(fn `RequestTurn`
  (bind _asbp_battle_game_mode (cast `/Game/Project/Blueprints/GameMode/BP_BattleGameMode` (`GameplayStatics.GetGameMode`)))
  (`/Game/Project/Blueprints/GameMode/BP_BattleGameMode.TurnRequest` _asbp_battle_game_mode (`self.UnitCharacter`)))

(fn `StartUnitTurn`
  (if (`KismetMathLibrary.ClassIsChildOf` (`GameplayStatics.GetObjectClass` (`self.UnitCharacter`)) "/Game/Project/Blueprints/SpriteUnit/PartySpriteBase.PartySpriteBase_C")
    (bind _returnvalue (`|CreateWidget` "/Game/Project/UI/Widget/UnitBattleHud.UnitBattleHud_C" null (`self.UnitCharacter`)))
    (bind _output_get (set `self.ActionCommandsWindow` _returnvalue))
    (`UserWidget.AddToViewport` _output_get 0)
    (else
      (bind _outactors (`GameplayStatics.GetAllActorsOfClass` "/Game/Project/Blueprints/SpriteUnit/PartySpriteBase.PartySpriteBase_C"))
      (set `self.UnitTarget` (`KismetArrayLibrary.Array_Random` _outactors))
      (switch `int` 0
        (:`0`
          (`self.AttackCommand`))))))