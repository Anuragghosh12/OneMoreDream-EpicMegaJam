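; Base sprite unit for battles that tracks HP and MP and reacts to damage with flipbook animations.
; On BeginPlay it derives HP and MP from the combat component's base stats and modifiers.
; Damage plays an optional hit reaction, applies the component's resistance calculation, shows a damage number widget, and at zero HP plays death and has BP_BattleGameMode remove the unit.
; SpendMP deducts clamped MP and fires MPSpent.
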(event `self.ReceiveBeginPlay`
  (bind _bp_combatcomponent (`self.BP_CombatComponent`))
  (bind ((`HP_2_7D215B4543E51324321261A9714AFE61` _hp) (`MP_9_E2BA56CD4E2554C38D28A0A07FA5E840` _mp)) (break `/Game/Project/Blueprints/SpriteUnits/Data/StatTableStruct` (`/Game/Project/Blueprints/GameMode/BP_CombatComponent.BaseUnitStats` _bp_combatcomponent)))
  (bind ((`HP_16_7D215B4543E51324321261A9714AFE61` _hp_2) (`MP_17_E2BA56CD4E2554C38D28A0A07FA5E840` _mp_2)) (break `/Game/Project/Blueprints/SpriteUnits/Data/StatModifier` (`/Game/Project/Blueprints/GameMode/BP_CombatComponent.UnitStatModifier` _bp_combatcomponent)))
  (`parent.ReceiveBeginPlay`)
  (bind _output_get (set `self.HP_Max` (* _hp _hp_2)))
  (set `self.HP_Current` _output_get)
  (bind _output_get_2 (set `self.MP_Max` (* _mp _mp_2)))
  (set `self.MP_Current` _output_get_2))

(event `self.ReceiveAnyDamage`
  (params (Damage :type "Float (single-precision)") (DamageType :type "DamageType Object Reference") (InstigatedBy :type "Controller Object Reference") (DamageCauser :type "Actor Object Reference"))
  (`|ExecutionSequence`
    (:`then_0`
      (bind _hitreact (`self.HitReact`)
        (:`then`
          (`PaperFlipbookComponent.SetFlipbook` (`self.Sprite`) _hitreact)
          (`KismetSystemLibrary.Delay` 0.6)
          (`PaperFlipbookComponent.SetFlipbook` (`self.Sprite`) (`self.Initial`)))
        (:`else`)))
    (:`then_1`
      (bind _newdamage (`/Game/Project/Blueprints/GameMode/BP_CombatComponent.CalculateDamageResistance` (`self.BP_CombatComponent`) Damage))
      (set `self.HP_Current` (`KismetMathLibrary.FClamp` (- (`self.HP_Current`) _newdamage) 0.0 (`self.HP_Max`)))
      (`|ExecutionSequence`
        (:`then_0`
          (bind _returnvalue (`|CreateWidget` "/Game/Project/UI/Widget/DamageNumber.DamageNumber_C" null _newdamage self))
          (`UserWidget.AddToViewport` _returnvalue 0))
        (:`then_1`
          (if (<= (`self.HP_Current`) 0.0)
            (`PaperFlipbookComponent.SetFlipbook` (`self.Sprite`) (`self.DeathAnim`))
            (`KismetSystemLibrary.Delay` 0.2)
            (bind _asbp_battle_game_mode (cast `/Game/Project/Blueprints/GameMode/BP_BattleGameMode` (`GameplayStatics.GetGameMode`)))
            (`/Game/Project/Blueprints/GameMode/BP_BattleGameMode.RemoveUnitFromBattle` _asbp_battle_game_mode self)))))))

(fn `SpendMP`
  (params (MPCost :type "Float (double-precision)"))
  (set `self.MP_Current` (`KismetMathLibrary.FClamp` (- (`self.MP_Current`) MPCost) 0.0 (`self.MP_Max`)))
  (`self.MPSpent`))

(fn `UserConstructionScript`
  (`parent.UserConstructionScript`)
  (set `self.Initial` (`PaperFlipbookComponent.GetFlipbook` (`self.Sprite`))))