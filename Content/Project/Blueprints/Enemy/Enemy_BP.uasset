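; Enemy pawn that roams randomly and chases the player after spotting them with PawnSensing.
; A seen player within a fixed range is followed via AIMoveTo; otherwise the enemy starts moving to its construction-time location, clears the sight flag and resumes roaming.
; Roaming moves to random reachable nearby points after a short delay, repeating only on success and switching to the follow logic if the sight flag is set.
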(event `self.ReceiveBeginPlay`
  (`self.Follow Player`))

(event `self.PawnSensing.OnSeePawn`
  (params (Pawn :type "Pawn Object Reference"))
  (set `self.IsSeeingPlayer` true)
  (`self.Follow Player`))

(event `Follow Player`
  (bind _returnvalue (`GameplayStatics.GetPlayerCharacter` 0))
  (if (`self.IsSeeingPlayer`)
    (if (<= (`self.GetDistanceTo` _returnvalue self) 360.0)
      (`|AIMoveTo` self (0.0 0.0 0.0) _returnvalue)
      (else
        (`|AIMoveTo` self (`self.Initial Location`) null
          (:`then`
            (set `self.IsSeeingPlayer` false)
            (`self.Random Roam`)))))
    (else
      (`self.Random Roam`))))

(event `Random Roam`
  (if (`self.IsSeeingPlayer`)
    (`self.Follow Player`)
    (else
      (`KismetSystemLibrary.Delay` 1.0)
      (`|AIMoveTo` self (`NavigationSystemV1.K2_GetRandomReachablePointInRadius` (`self.K2_GetActorLocation`) 200.0 null null) null
        (:`OnSuccess`
          (`self.Random Roam`))))))

(fn `UserConstructionScript`
  (set `self.Initial Location` (`self.K2_GetActorLocation`)))