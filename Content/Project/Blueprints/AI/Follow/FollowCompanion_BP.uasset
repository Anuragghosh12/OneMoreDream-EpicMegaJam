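; FollowCompanion_BP is a companion that follows the player character around using AI movement.
; On BeginPlay it casts and stores the player as MainPlayerCharacter_BP, then starts the FollowPlayer loop.
; FollowPlayer moves toward the player when at or beyond a short distance threshold, otherwise targets itself to halt.
; The loop re-triggers itself after a short Delay from each AIMoveTo's immediate output, polling instead of using Tick.
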(event `self.ReceiveBeginPlay`
  (bind _asmain_player_character_bp (cast `/Game/Project/Blueprints/MainPlayerCharacter_BP` (`GameplayStatics.GetPlayerCharacter` 0)))
  (set `self.As Main Player Character BP` _asmain_player_character_bp)
  (`self.FollowPlayer`))

(event `FollowPlayer`
  (if (>= (`self.GetDistanceTo` (`self.As Main Player Character BP`)) 100.0)
    (`|AIMoveTo` self (0.0 0.0 0.0) (`self.As Main Player Character BP`)
      (:`then`
        _))
    (else
      (`|AIMoveTo` self (0.0 0.0 0.0) self
        (:`then`
          _))))
  (`KismetSystemLibrary.Delay` 0.2)
  (`self.FollowPlayer`))

(fn `UserConstructionScript`
  (`parent.UserConstructionScript`))