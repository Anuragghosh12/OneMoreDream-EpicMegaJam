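; AI companion that follows the main player character and teleports to catch up when it falls behind.
; FollowPlayer issues AI move orders toward the player, or onto itself when close, then re-triggers itself and Teleport through short delays.
; Beyond a larger range, Teleport relocates it along the player's forward axis, scaled by distance and DistanceConstant, unless the player is falling.
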(event `self.ReceiveBeginPlay`
  ;[1 0.331 0.8496] Implementing Follow And Teleportation
  (bind _asmain_player_character_bp (cast `/Game/Project/Blueprints/MainPlayerCharacter_BP` (`GameplayStatics.GetPlayerCharacter` 0)))
  (set `self.As Main Player Character BP` _asmain_player_character_bp)
  (`self.Teleport`)
  (`self.FollowPlayer`))

(event `FollowPlayer`
  ;[0.208 0.3468 1] Character Follow Logic
  (if (>= (`self.GetDistanceTo` (`self.As Main Player Character BP`)) 100.0)
    (`|AIMoveTo` self (0.0 0.0 0.0) (`self.As Main Player Character BP`)
      (:`then`
        _))
    (else
      (`|AIMoveTo` self (0.0 0.0 0.0) self
        (:`then`
          _))))
  (`KismetSystemLibrary.Delay` 0.1)
  (`self.FollowPlayer`)
  (`KismetSystemLibrary.Delay` 0.2)
  (`self.Teleport`))

(event `Teleport`
  (bind _as_main_player_character_bp (`self.As Main Player Character BP`))
  (bind _as_main_player_character_bp_2 (`self.As Main Player Character BP`))
  (bind (_returnvalue_location _returnvalue_rotation) (`KismetMathLibrary.BreakTransform` (`self.GetTransform` _as_main_player_character_bp_2)))
  (bind _returnvalue_location_2 (`KismetMathLibrary.BreakTransform` (`KismetMathLibrary.MakeTransform` (+ _returnvalue_location (* (* (`self.GetActorForwardVector` _as_main_player_character_bp_2) (`self.GetDistanceTo` _as_main_player_character_bp_2)) (`self.Distance Constant`))) _returnvalue_rotation)))
  ;[1 0.2155 0.1538] Teleportation Logic
  (if (>= (`self.GetDistanceTo` _as_main_player_character_bp) 230.0)
    (if (not (`NavMovementComponent.IsFalling` (`Character.CharacterMovement` _as_main_player_character_bp)))
      (`self.K2_SetActorLocation` _returnvalue_location_2)
      (`self.FollowPlayer`))
    (else
      (`self.FollowPlayer`))))

(fn `UserConstructionScript`)