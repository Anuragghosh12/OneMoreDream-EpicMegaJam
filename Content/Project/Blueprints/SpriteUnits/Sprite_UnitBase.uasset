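; Base Blueprint for sprite units that flashes a hit-reaction flipbook when the unit takes damage.
; The construction script caches the Sprite component's current flipbook as Initial.
; On any damage, a valid HitReact flipbook replaces it for a half-second delay, then Initial is restored.
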(event `self.ReceiveBeginPlay`
  (`parent.ReceiveBeginPlay`))

(event `self.ReceiveAnyDamage`
  (params (Damage :type "Float (single-precision)") (DamageType :type "DamageType Object Reference") (InstigatedBy :type "Controller Object Reference") (DamageCauser :type "Actor Object Reference"))
  (bind _hitreact (`self.HitReact`)
    (:`then`
      (`PaperFlipbookComponent.SetFlipbook` (`self.Sprite`) _hitreact)
      (`KismetSystemLibrary.Delay` 0.5)
      (`PaperFlipbookComponent.SetFlipbook` (`self.Sprite`) (`self.Initial`)))
    (:`else`)))

(fn `UserConstructionScript`
  (`parent.UserConstructionScript`)
  (set `self.Initial` (`PaperFlipbookComponent.GetFlipbook` (`self.Sprite`))))